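; BP_BasicPlayerState is a player state that stores the player's picked-up equipment in the PickUpInfo array and mirrors it to the backpack widget.
; UpdataeCoalescing uses FindItemWithId to search by InfoID and appends unmatched items as new lattice entries.
; On a match, it checks CanOverlap on element 0, not the found index, then either adds to that element's Count or appends a new entry.
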(fn `FindItemWithId`
  (params (PickUpInfo :type "/Game/ColdWinterWind/Blueprint/Struct/Interactable/EquipmentInfo Structure"))
  (returns (Index :type Integer))
  (for (_array_element _array_index) (`self.PickUpInfo`)
    (if (== (`.InfoID_35_9F58E16248EE604E946007B05449FEB0` (break `/Game/ColdWinterWind/Blueprint/Struct/Interactable/EquipmentInfo` _array_element)) (`.InfoID_35_9F58E16248EE604E946007B05449FEB0` (break `/Game/ColdWinterWind/Blueprint/Struct/Interactable/EquipmentInfo` PickUpInfo)))
      (return _array_index)))
  (return -1))

(fn `UpdataeCoalescing`
  (params (Equipmentinfo :type "/Game/ColdWinterWind/Blueprint/Struct/Interactable/EquipmentInfo Structure") (LoadWidget :type "/Game/ColdWinterWind/Blueprint/BP-Widget/LordUI Object Reference"))
  (bind _backpackwidget (`/Game/ColdWinterWind/Blueprint/BP-Widget/LordUI.BackpackWidget` LoadWidget))
  (bind _pickupinfo (`self.PickUpInfo`))
  (bind _pickupinfo_2 (`self.PickUpInfo`))
  (bind _output (`|GetArrayItem` (`self.PickUpInfo`)))
  (bind (_infoid _isvalid_ _index _name _image _category _type _property _count _canoverlap_) (break `/Game/ColdWinterWind/Blueprint/Struct/Interactable/EquipmentInfo` _output))
  (if (< (`self.FindItemWithId` Equipmentinfo) 0)
    (bind _returnvalue (`KismetArrayLibrary.Array_Add` _pickupinfo Equipmentinfo))
    (`/Game/ColdWinterWind/Blueprint/BP-Widget/BackpackWidget.AddToLatticeWiget` (`/Game/ColdWinterWind/Blueprint/BP-Widget/LordUI.BackpackWidget` LoadWidget) (`|GetArrayItem` _pickupinfo _returnvalue))
    (elif _canoverlap_
      (bind _structout (setmembers `/Game/ColdWinterWind/Blueprint/Struct/Interactable/EquipmentInfo` :`StructRef` _output :`Count` (+ _count (`.Count_23_B31E1D2E46C33F5B98BDE5AA19AFA1DD` (break `/Game/ColdWinterWind/Blueprint/Struct/Interactable/EquipmentInfo` Equipmentinfo)))))
      (`/Game/ColdWinterWind/Blueprint/BP-Widget/BackpackWidget.UpdatePickUpInfo` _backpackwidget _structout)
      (else
        (bind _returnvalue_2 (`KismetArrayLibrary.Array_Add` _pickupinfo_2 Equipmentinfo))
        (`/Game/ColdWinterWind/Blueprint/BP-Widget/BackpackWidget.AddToLatticeWiget` _backpackwidget (`|GetArrayItem` _pickupinfo_2 _returnvalue_2))))))

(fn `UserConstructionScript`)