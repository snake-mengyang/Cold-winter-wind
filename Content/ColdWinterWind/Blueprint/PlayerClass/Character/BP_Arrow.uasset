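; BP_Arrow is an arrow actor that delivers an attack to whatever it overlaps.
; When its capsule overlaps an actor other than its instigator that implements BPI_AttackState, it sends AttackMessage with attack type, damage and its own location as the hit point, then destroys itself.
; Overlaps with other actors are ignored, and the arrow destroys itself after a short fixed lifetime from BeginPlay.
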(event `self.ReceiveBeginPlay`
  (`KismetSystemLibrary.Delay` 4.0)
  (`self.K2_DestroyActor`))

(event `self.Capsule.OnComponentBeginOverlap`
  (params (OverlappedComponent :type "PrimitiveComponent Object Reference") (OtherActor :type "Actor Object Reference") (OtherComp :type "PrimitiveComponent Object Reference") (OtherBodyIndex :type Integer) (bFromSweep :type Boolean) (SweepResult :type "HitResult Structure (by ref)"))
  (if (and (!= (`self.Instigator`) OtherActor) (`KismetSystemLibrary.DoesImplementInterface` OtherActor "/Game/ColdWinterWind/Blueprint/Interface/BPI_AttackState.BPI_AttackState_C"))
    (message `/Game/ColdWinterWind/Blueprint/Interface/BPI_AttackState.Attack` OtherActor (`self.AttackType`) (`self.Damge`) (`self.K2_GetActorLocation`))
    (`self.K2_DestroyActor`)))

(fn `UserConstructionScript`)