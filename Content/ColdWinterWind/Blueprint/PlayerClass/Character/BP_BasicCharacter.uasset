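; Player character Blueprint handling item interaction, equipment drops, backpack UI updates and skill combo montages.
; Each tick it highlights the registered interactable best aligned with the camera via dot product, storing it on the player state.
; Drops spawn physics-simulated BP_HelmEquipment; pickups go to the backpack widget.
; Active skills play main montages, while trigger skills queue follow-up sections around a notify-opened combo window, with keyboard-widget highlights and cooldowns.
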(event `self.ReceiveBeginPlay`
  (bind _asbp_basic_player_state (cast `/Game/ColdWinterWind/Blueprint/PlayerClass/PlayerState/BP_BasicPlayerState` (`self.PlayerState`)))
  (set `self.StateRef` _asbp_basic_player_state)
  (bind _asbasic_character_anim (cast `/Game/ColdWinterWind/Blueprint/AnimBP/BasicCharacter_Anim` (`SkeletalMeshComponent.GetAnimInstance` (`self.Mesh`))))
  (set `self.AnimBPRef` _asbasic_character_anim)
  (bind _asbp_basic_player_controller (cast `/Game/ColdWinterWind/Blueprint/PlayerClass/PlayerController/BP_BasicPlayerController` (`self.GetController`)))
  (set `self.ControllerRef` _asbp_basic_player_controller))

(event `self.ReceiveTick`
  (params (DeltaSeconds :type "Float (single-precision)"))
  (`self.UpdateBestInteractable`))

(event `/Game/ColdWinterWind/Blueprint/Interface/BPI_Interactable.RegisterInteractable`
  (params (Interactable :type "/Game/ColdWinterWind/Blueprint/InteractableClass/BP_BaseInteractable Object Reference"))
  (`self.HandleRegisterInteractable` Interactable))

(event `/Game/ColdWinterWind/Blueprint/Interface/BPI_Interactable.UnReginsterInteractable`
  (params (Interactable :type "/Game/ColdWinterWind/Blueprint/InteractableClass/BP_BaseInteractable Object Reference"))
  (`self.HandleUnRegisterInteractable` Interactable))

(event `DropInteractable`
  (params (PickUpInfo :type "/Game/ColdWinterWind/Blueprint/Struct/Interactable/EquipmentInfo Structure"))
  (`KismetArrayLibrary.Array_RemoveItem` (`/Game/ColdWinterWind/Blueprint/PlayerClass/PlayerState/BP_BasicPlayerState.PickUpInfo` (`self.StateRef`)) PickUpInfo)
  (bind _structout (setmembers `/Game/ColdWinterWind/Blueprint/Struct/Interactable/EquipmentInfo` :`StructRef` PickUpInfo :`Index` 0))
  (bind _returnvalue (`|SpawnActorFromClass` "/Game/ColdWinterWind/Blueprint/InteractableClass/Equipment/BP_HelmEquipment.BP_HelmEquipment_C" (`SceneComponent.K2_GetComponentToWorld` (`self.DropInfoOrigin`)) "Undefined" "OverrideRootScale" null _structout null))
  (`PrimitiveComponent.SetSimulatePhysics` (`/Game/ColdWinterWind/Blueprint/InteractableClass/BP_BaseInteractable.InteractableMesh` _returnvalue) true))

(event `ForFindBackLocation`
  (params (PickUpInfo :type "/Game/ColdWinterWind/Blueprint/Struct/Interactable/EquipmentInfo Structure"))
  (bind _asbp_basic_player_controller (cast `/Game/ColdWinterWind/Blueprint/PlayerClass/PlayerController/BP_BasicPlayerController` (`self.GetController`)))
  (bind _backpackwidget (`/Game/ColdWinterWind/Blueprint/BP-Widget/LordUI.BackpackWidget` (`/Game/ColdWinterWind/Blueprint/PlayerClass/PlayerController/BP_BasicPlayerController.LordUI` _asbp_basic_player_controller)))
  (`/Game/ColdWinterWind/Blueprint/BP-Widget/BackpackWidget.AddToLatticeWiget` _backpackwidget PickUpInfo)
  (`/Game/ColdWinterWind/Blueprint/BP-Widget/BackpackWidget.RefreshBack` _backpackwidget))

(event `CharacterPlayMontage`
  (params (SkillInfo :type "/Game/ColdWinterWind/Blueprint/BP-Widget/KeybordUMG/KeybordItemWidget Object Reference"))
  (bind (_isvalid_ _skillname _skilltexture _skilltype) (break `/Game/ColdWinterWind/Blueprint/Struct/Skill/SkillInfo` (`/Game/ColdWinterWind/Blueprint/BP-Widget/KeybordUMG/KeybordItemWidget.SkillInfo` SkillInfo)))
  (if _isvalid_
    (switch `/Game/ColdWinterWind/Blueprint/Enum/Skill/E_SkillType` _skilltype
      (:`NewEnumerator0`
        (if (not (`self.IsPlayerMontage?`))
          (set `self.MainSkillKeyboard` SkillInfo)
          (set `self.IsPlayerMontage?` true)
          (set `self.CanCombination` false)
          (set `self.Combinationed?` false)
          (`/Game/ColdWinterWind/Blueprint/BP-Widget/KeybordUMG/KeybordWidget.SecondaryHighLight` (`/Game/ColdWinterWind/Blueprint/BP-Widget/LordUI.KeybordWidget` (`/Game/ColdWinterWind/Blueprint/PlayerClass/PlayerController/BP_BasicPlayerController.LordUI` (`self.ControllerRef`))))
          (`|PlayMontage` (`self.Mesh`) (`BlueprintMapLibrary.Map_Find` (`self.MainMontageMap`) _skillname)
            (:`OnCompleted`
              (if (not (`self.Combinationed?`))
                (`/Game/ColdWinterWind/Blueprint/BP-Widget/KeybordUMG/KeybordItemWidget.SkillCD` (`self.MainSkillKeyboard`)))
              (set `self.Combinationed?` false)
              (set `self.IsPlayerMontage?` false)
              (`/Game/ColdWinterWind/Blueprint/BP-Widget/KeybordUMG/KeybordWidget.SecondaryNotHighLight` (`/Game/ColdWinterWind/Blueprint/BP-Widget/LordUI.KeybordWidget` (`/Game/ColdWinterWind/Blueprint/PlayerClass/PlayerController/BP_BasicPlayerController.LordUI` (`self.ControllerRef`)))))
            (:`OnNotifyBegin`
              (set `self.CanCombination` true)
              (if (`self.Combinationed?`)
                (set `self.CanCombination` false)
                (`|PlayMontage` (`self.Mesh`) "/Game/ColdWinterWind/Animation/Montage/AttackFollowUp_Montage.AttackFollowUp_Montage" 1.0 0.0 (`self.NextMontageName`)
                  (:`OnCompleted`
                    (set `self.IsPlayerMontage?` false)
                    (`/Game/ColdWinterWind/Blueprint/BP-Widget/KeybordUMG/KeybordItemWidget.SkillCD` (`self.MainSkillKeyboard`)))))))))
      (:`NewEnumerator1`
        (if (`self.CanCombination`)
          (`/Game/ColdWinterWind/Blueprint/BP-Widget/KeybordUMG/KeybordWidget.SecondaryNotHighLight` (`/Game/ColdWinterWind/Blueprint/BP-Widget/LordUI.KeybordWidget` (`/Game/ColdWinterWind/Blueprint/PlayerClass/PlayerController/BP_BasicPlayerController.LordUI` (`self.ControllerRef`))))
          (if (`self.Combinationed?`)
            (set `self.Combinationed?` false)
            (`|PlayMontage` (`self.Mesh`) "/Game/ColdWinterWind/Animation/Montage/AttackFollowUp_Montage.AttackFollowUp_Montage" 1.0 0.0 (`BlueprintMapLibrary.Map_Find` (`self.SecondaryMontageMap`) _skillname)
              (:`OnCompleted`
                (set `self.IsPlayerMontage?` false)
                (set `self.Combinationed?` false)
                (`/Game/ColdWinterWind/Blueprint/BP-Widget/KeybordUMG/KeybordItemWidget.SkillCD` (`self.MainSkillKeyboard`)))))
          (else
            (set `self.NextMontageName` (`BlueprintMapLibrary.Map_Find` (`self.SecondaryMontageMap`) _skillname))
            (set `self.Combinationed?` true)
            (`/Game/ColdWinterWind/Blueprint/BP-Widget/KeybordUMG/KeybordWidget.SecondaryNotHighLight` (`/Game/ColdWinterWind/Blueprint/BP-Widget/LordUI.KeybordWidget` (`/Game/ColdWinterWind/Blueprint/PlayerClass/PlayerController/BP_BasicPlayerController.LordUI` (`self.ControllerRef`))))))))))

(fn `GetBestInteractable`
  (locals (InteractableVerialble :type "/Game/ColdWinterWind/Blueprint/Struct/Interactable/FInteractableVariable Structure"))
  (bind _followcamera (`self.FollowCamera`))
  (bind _interactableverialble_dot (break `/Game/ColdWinterWind/Blueprint/Struct/Interactable/FInteractableVariable` (`local.InteractableVerialble`)))
  (bind (_interactableverialble_dot_2 _interactableverialble_interactable) (break `/Game/ColdWinterWind/Blueprint/Struct/Interactable/FInteractableVariable` (`local.InteractableVerialble`)))
  (set `local.InteractableVerialble` (make `/Game/ColdWinterWind/Blueprint/Struct/Interactable/FInteractableVariable` -1.0))
  (for _array_element (`/Game/ColdWinterWind/Blueprint/PlayerClass/PlayerState/BP_BasicPlayerState.Interactables` (`self.StateRef`))
    (bind _returnvalue (`KismetMathLibrary.Dot_VectorVector` (`KismetMathLibrary.Normal` (- (`PrimitiveComponent.GetCenterOfMass` (`/Game/ColdWinterWind/Blueprint/InteractableClass/BP_BaseInteractable.InteractableMesh` _array_element) "None") (`SceneComponent.K2_GetComponentLocation` _followcamera))) (`SceneComponent.GetForwardVector` _followcamera)))
    (if (and (> _returnvalue 0.8) (> _returnvalue _interactableverialble_dot))
      (set `local.InteractableVerialble` (make `/Game/ColdWinterWind/Blueprint/Struct/Interactable/FInteractableVariable` _returnvalue _array_element))))
  (`/Engine/EditorBlueprintResources/StandardMacros.IsValid` _interactableverialble_interactable
    (:`Is Valid`
      (`self.SetBestInteractable` _interactableverialble_interactable))
    (:`Is Not Valid`
      (`self.SetBestInteractable` null))))

(fn `HandleRegisterInteractable`
  (params (Interactable :type "/Game/ColdWinterWind/Blueprint/InteractableClass/BP_BaseInteractable Object Reference"))
  (`KismetArrayLibrary.Array_AddUnique` (`/Game/ColdWinterWind/Blueprint/PlayerClass/PlayerState/BP_BasicPlayerState.Interactables` (`self.StateRef`)) Interactable))

(fn `HandleUnRegisterInteractable`
  (params (Interactable :type "/Game/ColdWinterWind/Blueprint/InteractableClass/BP_BaseInteractable Object Reference"))
  (`KismetArrayLibrary.Array_RemoveItem` (`/Game/ColdWinterWind/Blueprint/PlayerClass/PlayerState/BP_BasicPlayerState.Interactables` (`self.StateRef`)) Interactable))

(fn `SetBestInteractable`
  (params (Interactable :type "/Game/ColdWinterWind/Blueprint/InteractableClass/BP_BaseInteractable Object Reference"))
  (bind _stateref (`self.StateRef`))
  (bind _stateref_2 (`self.StateRef`))
  (`/Engine/EditorBlueprintResources/StandardMacros.IsValid` Interactable
    (:`Is Valid`
      (if (!= Interactable (`/Game/ColdWinterWind/Blueprint/PlayerClass/PlayerState/BP_BasicPlayerState.HighLightedInteractable` _stateref))
        (bind _highlightedinteractable (`/Game/ColdWinterWind/Blueprint/PlayerClass/PlayerState/BP_BasicPlayerState.HighLightedInteractable` _stateref_2)
          (:`then`
            (`/Game/ColdWinterWind/Blueprint/InteractableClass/BP_BaseInteractable.SetHighLight` _highlightedinteractable false))
          (:`else`
            _)))
      (bind _output_get (set `/Game/ColdWinterWind/Blueprint/PlayerClass/PlayerState/BP_BasicPlayerState.HighLightedInteractable` Interactable _stateref_2))
      (`/Game/ColdWinterWind/Blueprint/InteractableClass/BP_BaseInteractable.SetHighLight` _output_get true))
    (:`Is Not Valid`
      (bind _highlightedinteractable_2 (`/Game/ColdWinterWind/Blueprint/PlayerClass/PlayerState/BP_BasicPlayerState.HighLightedInteractable` _stateref)
        (:`then`
          (`/Game/ColdWinterWind/Blueprint/InteractableClass/BP_BaseInteractable.SetHighLight` _highlightedinteractable_2 false)
          (set `/Game/ColdWinterWind/Blueprint/PlayerClass/PlayerState/BP_BasicPlayerState.HighLightedInteractable` null (`self.StateRef`)))
        (:`else`)))))

(fn `UpdateBestInteractable`
  (if (> (`KismetArrayLibrary.Array_Length` (`/Game/ColdWinterWind/Blueprint/PlayerClass/PlayerState/BP_BasicPlayerState.Interactables` (`self.StateRef`))) 0)
    (`self.GetBestInteractable`)
    (else
      (`self.SetBestInteractable` null))))

(fn `UserConstructionScript`)