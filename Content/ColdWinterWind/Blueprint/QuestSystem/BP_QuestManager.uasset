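; Quest manager that starts, tracks and completes quests from QuestTable, sorting unfinished and completed rows in its construction script.
; BeginQuestInfo turns an unclaimed quest into a QuestWidget in the UI list; these widgets serve as the running-quest records.
; CheckCurrentQuest highlights the selected quest and updates the LordWidgetRef display, while QuestToggle cycles selection.
; CompleteGoal advances sub-goals, then loads the follow-up quest into the same widget or records completion.
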(event `self.ReceiveBeginPlay`)

(event `self.ReceiveActorBeginOverlap`
  (params (OtherActor :type "Actor Object Reference")))

(fn `BeginQuestInfo`
  (params (QuestName :type Name))
  (bind _returnvalue (`|GetDataTableRow` "/Game/ColdWinterWind/DataTable/QuestTable.QuestTable" QuestName)
    (:`then`
      (if (`|EnumEquality` (`.QuestType_31_F1D0F39F49ACECB90F37CC865CA46341` (break `/Game/ColdWinterWind/Blueprint/Struct/Quest/QuestInfo` _returnvalue)) "NewEnumerator3")
        (`self.CreateQuestWidget` _returnvalue)))))

(fn `CheckCurrentQuest`
  (params (CurrentIndex :type Integer))
  (for (_array_element _array_index) (`self.RunningQuests`)
    (if (== _array_index CurrentIndex)
      (bind _initiatorarr (`/Game/ColdWinterWind/Blueprint/BP-Widget/QuestUMG/QuestWidget.SelectToCurrentQuest` _array_element))
      (set `self.CurrentQuestIndex` _array_index)
      (`/Game/ColdWinterWind/Blueprint/BP-Widget/LordUI.UpdateChattingWiget` (`self.LordWidgetRef`) _initiatorarr)
      (else
        (`/Game/ColdWinterWind/Blueprint/BP-Widget/QuestUMG/QuestWidget.RemoveToCurrentQuest` _array_element)))))

(fn `CompleteGoal`
  (bind _returnvalue (+ (`self.CurrentQuestIndex`) 1))
  (bind _output (`|GetArrayItem` (`self.RunningQuests`) (`self.CurrentQuestIndex`)))
  (bind (_name _category _description _region _area _suggestedlevel _completionreward _currentgoalindex _subgoals _questtype _hassubsequent _subsequentquestname) (break `/Game/ColdWinterWind/Blueprint/Struct/Quest/QuestInfo` (`/Game/ColdWinterWind/Blueprint/BP-Widget/QuestUMG/QuestWidget.QuestInfo` _output)))
  (bind _completequest_ (`/Game/ColdWinterWind/Blueprint/BP-Widget/QuestUMG/QuestWidget.CompleteSubGoal` _output))
  (`self.CheckCurrentQuest` (`self.CurrentQuestIndex`))
  (if _completequest_
    (if _hassubsequent
      (bind _returnvalue_2 (`|GetDataTableRow` "/Game/ColdWinterWind/DataTable/QuestTable.QuestTable" _subsequentquestname)
        (:`then`
          (set `/Game/ColdWinterWind/Blueprint/BP-Widget/QuestUMG/QuestWidget.QuestInfo` _returnvalue_2 _output)
          (`/Game/ColdWinterWind/Blueprint/BP-Widget/QuestUMG/QuestWidget.UpdateQuestInfo` _output)
          (`self.CheckCurrentQuest` (`self.CurrentQuestIndex`))))
      (else
        (`Widget.RemoveFromParent` _output)
        (bind _structout (setmembers `/Game/ColdWinterWind/Blueprint/Struct/Quest/QuestInfo` :`StructRef` (`/Game/ColdWinterWind/Blueprint/BP-Widget/QuestUMG/QuestWidget.QuestInfo` _output) :`QuestType` "NewEnumerator2"))
        (`KismetArrayLibrary.Array_AddUnique` (`self.CompletedQuests`) _structout)
        (if (< _returnvalue (`KismetArrayLibrary.Array_Length` (`self.RunningQuests`)))
          (bind _output_get (set `self.CurrentQuestIndex` _returnvalue))
          (`self.CheckCurrentQuest` _output_get))))))

(fn `CreateQuestWidget`
  (params (InputPin :type "/Game/ColdWinterWind/Blueprint/Struct/Quest/QuestInfo Structure"))
  (bind _returnvalue (`|CreateWidget` "/Game/ColdWinterWind/Blueprint/BP-Widget/QuestUMG/QuestWidget.QuestWidget_C" null InputPin))
  (bind _returnvalue_2 (`KismetArrayLibrary.Array_AddUnique` (`self.RunningQuests`) _returnvalue))
  (`PanelWidget.AddChild` (`/Game/ColdWinterWind/Blueprint/BP-Widget/LordUI.QuestList` (`/Game/ColdWinterWind/Blueprint/PlayerClass/PlayerController/BP_BasicPlayerController.LordUI` (`self.CharacterControllerRef`))) _returnvalue)
  (bind _output_get (set `self.CurrentQuestIndex` _returnvalue_2))
  (`self.CheckCurrentQuest` _output_get))

(fn `QuestToggle`
  (bind _returnvalue (+ (`self.CurrentQuestIndex`) 1))
  (if (< _returnvalue (`KismetArrayLibrary.Array_Length` (`self.RunningQuests`)))
    (`self.CheckCurrentQuest` _returnvalue)
    (else
      (bind _output_get (set `self.CurrentQuestIndex` 0))
      (`self.CheckCurrentQuest` _output_get))))

(fn `UserConstructionScript`
  (locals (QuestInfo :type "/Game/ColdWinterWind/Blueprint/Struct/Quest/QuestInfo Structure"))
  (bind _outrownames (`DataTableFunctionLibrary.GetDataTableRowNames` "/Game/ColdWinterWind/DataTable/QuestTable.QuestTable"))
  (for _array_element _outrownames
    (bind _returnvalue (`|GetDataTableRow` "/Game/ColdWinterWind/DataTable/QuestTable.QuestTable" _array_element)
      (:`then`
        (switch `/Game/ColdWinterWind/Blueprint/Enum/Quest/E_QuestType` (`.QuestType_31_F1D0F39F49ACECB90F37CC865CA46341` (break `/Game/ColdWinterWind/Blueprint/Struct/Quest/QuestInfo` _returnvalue))
          (:`NewEnumerator0`
            (`KismetArrayLibrary.Array_AddUnique` (`self.NotCompletedQuests`) _returnvalue))
          (:`NewEnumerator2`
            (`KismetArrayLibrary.Array_AddUnique` (`self.CompletedQuests`) _returnvalue)))))))