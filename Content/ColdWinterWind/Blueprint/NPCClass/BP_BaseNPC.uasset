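; BP_BaseNPC is a base NPC that patrols and detects the player, driven by a behavior tree.
; On BeginPlay it runs the tree and seeds the blackboard with its starting location and patrol radius.
; A sphere overlap flags the player pawn as seen on the blackboard.
; Any BP_BasicCharacter leaving the sphere clears that flag and finishes the referenced task; player-object and walk-speed nodes are unconnected.
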(event `self.ReceiveBeginPlay`
  (bind _returnvalue (`AIBlueprintHelperLibrary.GetBlackboard` null))
  (`AIController.RunBehaviorTree` (`AIBlueprintHelperLibrary.GetAIController` self) (`self.BehaviourTree`))
  (`BlackboardComponent.SetValueAsVector` _returnvalue "OriginalLocation" (`self.K2_GetActorLocation`))
  (`BlackboardComponent.SetValueAsFloat` _returnvalue "PatrolRadius" (`self.PatrolRadius`)))

(event `self.Sphere.OnComponentBeginOverlap`
  (params (OverlappedComponent :type "PrimitiveComponent Object Reference") (OtherActor :type "Actor Object Reference") (OtherComp :type "PrimitiveComponent Object Reference") (OtherBodyIndex :type Integer) (bFromSweep :type Boolean) (SweepResult :type "HitResult Structure (by ref)"))
  (bind _asbp_basic_character (cast `/Game/ColdWinterWind/Blueprint/PlayerClass/Character/BP_BasicCharacter` OtherActor))
  (if (and (== _asbp_basic_character (`GameplayStatics.GetPlayerPawn` 0)) (not (`self.HasSeenPlayer?`)))
    (set `self.HasSeenPlayer?` true)
    (`BlackboardComponent.SetValueAsBool` (`AIBlueprintHelperLibrary.GetBlackboard` null) "HasSeenPlayer?" true)))

(event `self.Sphere.OnComponentEndOverlap`
  (params (OverlappedComponent :type "PrimitiveComponent Object Reference") (OtherActor :type "Actor Object Reference") (OtherComp :type "PrimitiveComponent Object Reference") (OtherBodyIndex :type Integer))
  (cast `/Game/ColdWinterWind/Blueprint/PlayerClass/Character/BP_BasicCharacter` OtherActor)
  (set `self.HasSeenPlayer?` false)
  (`BlackboardComponent.SetValueAsBool` (`AIBlueprintHelperLibrary.GetBlackboard` null) "HasSeenPlayer?" false)
  (`BTTask_BlueprintBase.FinishExecute` (`self.TaskRef`) true))

(fn `UserConstructionScript`)