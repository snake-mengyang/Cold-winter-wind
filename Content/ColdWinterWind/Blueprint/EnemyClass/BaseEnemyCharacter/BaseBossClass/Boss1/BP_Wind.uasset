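; Short-lived wind hazard pawn, filed under Boss1, that chases the player and damages them on contact.
; On spawn it AI-moves to a random nearby navigable point, then repeatedly re-targets the player's location, while a parallel delay destroys it.
; Capsule overlap with a BP_BasicCharacter sends AttackMessage immediately and on a looping timer, which is cleared when the overlap ends.
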(event `self.ReceiveBeginPlay`
  (`|ExecutionSequence`
    (:`then_0`
      (`|AIMoveTo` self (`NavigationSystem.K2_GetRandomLocationInNavigableRadius` (`self.K2_GetActorLocation`) 500.0)
        (:`OnSuccess`
          _)
        (:`OnFail`
          _))
      (`|AIMoveTo` self (`self.K2_GetActorLocation` (`GameplayStatics.GetPlayerCharacter` 0)) :!label _label
        (:`OnSuccess`
          _)
        (:`OnFail`
          _))
      (`KismetSystemLibrary.Delay` 0.2)
      (goto _label))
    (:`then_1`
      (`KismetSystemLibrary.Delay` 15.0)
      (`self.K2_DestroyActor`))))

(event `self.Capsule.OnComponentBeginOverlap`
  (params (OverlappedComponent :type "PrimitiveComponent Object Reference") (OtherActor :type "Actor Object Reference") (OtherComp :type "PrimitiveComponent Object Reference") (OtherBodyIndex :type Integer) (bFromSweep :type Boolean) (SweepResult :type "HitResult Structure (by ref)"))
  (bind _returnvalue (`self.K2_GetActorLocation`))
  (bind _asbp_basic_character (cast `/Game/ColdWinterWind/Blueprint/PlayerClass/Character/BP_BasicCharacter` OtherActor))
  (bind _output_get (set `self.PlayerRef` _asbp_basic_character))
  (message `/Game/ColdWinterWind/Blueprint/Interface/BPI_AttackState.Attack` _output_get "NewEnumerator0" -5.0 _returnvalue null false _returnvalue)
  (bind _returnvalue_2 (`KismetSystemLibrary.K2_SetTimerDelegate` (delegate `HandleAttack`) 2.0 true))
  (set `self.HandleAttackRef` _returnvalue_2))

(event `HandleAttack`
  (bind _returnvalue (`self.K2_GetActorLocation`))
  (message `/Game/ColdWinterWind/Blueprint/Interface/BPI_AttackState.Attack` (`self.PlayerRef`) "NewEnumerator0" -5.0 _returnvalue null false _returnvalue))

(event `self.Capsule.OnComponentEndOverlap`
  (params (OverlappedComponent :type "PrimitiveComponent Object Reference") (OtherActor :type "Actor Object Reference") (OtherComp :type "PrimitiveComponent Object Reference") (OtherBodyIndex :type Integer))
  (cast `/Game/ColdWinterWind/Blueprint/PlayerClass/Character/BP_BasicCharacter` OtherActor)
  (set `self.PlayerRef` null)
  (`KismetSystemLibrary.K2_ClearAndInvalidateTimerHandle` (`self.HandleAttackRef`)))

(fn `UserConstructionScript`)