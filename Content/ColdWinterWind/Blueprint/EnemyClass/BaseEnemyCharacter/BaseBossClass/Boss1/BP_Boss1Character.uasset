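; First boss enemy character: sight perception reports the player to its AI controller, and behavior tree tasks call its montage events, which finish the task when done.
; Incoming hits reduce HP and write death or hit-reaction blackboard keys, with reactions and attacker attachment suppressed during attacks.
; GetBehaviorStatus randomly picks attack or move montages, weighted by missing HP and player fall state.
; ReleaseMagic spawns wind, fire circle or triple player-tracking lightning.
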(event `self.ReceiveBeginPlay`
  (`parent.ReceiveBeginPlay`)
  (bind _asbp_boss_1aicontroller (cast `/Game/ColdWinterWind/Blueprint/EnemyClass/BaseEnemyAIController/BaseBossAIController/Boos1/BP_Boss1AIController` (`self.GetController`)))
  (set `self.AIControllerRef` _asbp_boss_1aicontroller))

(event `BehaviorMontage`
  (params (Montage :type "AnimMontage Object Reference") (Name :type Name) (BTTask :type "/Game/ColdWinterWind/Blueprint/EnemyClass/BaseEnemyBehaviorTree/Boss1/BTT_Execution Object Reference"))
  (if (== Montage "/Game/ColdWinterWind/Animation/Montage/Enemy/Boss/AttackMontage.AttackMontage")
    (set `self.IsAttack?` true))
  (`|PlayMontage` (`self.Mesh`) Montage 1.0 0.0 Name
    (:`OnCompleted`
      _)
    (:`OnInterrupted`
      _))
  (set `self.IsAttack?` false)
  (`BTTask_BlueprintBase.FinishExecute` BTTask true))

(event `PlayFindEnemyMontage`
  (params (BTTTask :type "BTTask_BlueprintBase Object Reference") (`Success?` :type Boolean))
  (`|PlayMontage` (`self.Mesh`) "/Game/ColdWinterWind/Animation/Montage/Enemy/Boss/StatusMontage.StatusMontage" 1.0 0.0 "Find"
    (:`OnCompleted`
      _)
    (:`OnInterrupted`
      _))
  (if (not `Success?`)
    (`BlackboardComponent.SetValueAsBool` (`AIBlueprintHelperLibrary.GetBlackboard` null) "IsRoar?" true))
  (`BTTask_BlueprintBase.FinishExecute` BTTTask `Success?`))

(event `AttackType`
  (params (AttackType :type "/Game/ColdWinterWind/Blueprint/Enum/E_Attack Enum" :default "NewEnumerator0") (Damage :type "Float (double-precision)") (`IsAttach?` :type Boolean))
  (`self.AttackToOther` AttackType (`SceneComponent.K2_GetComponentLocation` (`self.WeaponOrigin`)) Damage `IsAttach?`))

(event `self.AIPerception.OnTargetPerceptionUpdated`
  (params (Actor :type "Actor Object Reference") (Stimulus :type "AIStimulus Structure"))
  (bind _returnvalue (`AIPerceptionSystem.GetSenseClassForStimulus` Stimulus))
  (if (and (== _returnvalue "/Script/AIModule.AISense_Sight") (`.bSuccessfullySensed` (break `AIStimulus` Stimulus)))
    (bind _asbp_basic_character (cast `/Game/ColdWinterWind/Blueprint/PlayerClass/Character/BP_BasicCharacter` Actor))
    (`/Game/ColdWinterWind/Blueprint/EnemyClass/BaseEnemyAIController/BaseBossAIController/Boos1/BP_Boss1AIController.FindPlayer` (`self.AIControllerRef`) _asbp_basic_character)))

(event `/Game/ColdWinterWind/Blueprint/Interface/BPI_AttackState.Attack`
  (params (AttackType :type "/Game/ColdWinterWind/Blueprint/Enum/E_Attack Enum" :default "NewEnumerator0") (Damage :type "Float (single-precision)") (HitLocation :type "Vector Structure") (SelfRef :type "Character Object Reference") (`IsAttach?` :type Boolean) (HitWhere :type "Vector Structure"))
  (bind _returnvalue (`AIBlueprintHelperLibrary.GetBlackboard` null))
  (bind _returnvalue_2 (- (`self.HP`) Damage))
  (cast `/Game/ColdWinterWind/Blueprint/PlayerClass/Character/BP_BasicCharacter` SelfRef
    (:`then`
      (`GameplayStatics.SpawnEmitterAtLocation` "/Game/ColdWinterWind/ParticleSystem/AdvancedMagicFX10/P_AttackStatus.P_AttackStatus" HitWhere (`self.K2_GetActorRotation`) (0.5 0.5 0.5)))
    (:`CastFailed`
      _))
  (if (<= _returnvalue_2 0.0)
    (`BlackboardComponent.SetValueAsBool` (`AIBlueprintHelperLibrary.GetBlackboard` null) "Death?" true)
    (else
      (set `self.HP` _returnvalue_2)
      (if (not (`self.IsAttack?`))
        (if `IsAttach?`
          (`self.K2_AttachToActor` SelfRef "None" "KeepWorld" "KeepWorld" "KeepWorld")
          (else
            (`self.K2_DetachFromActor` "KeepWorld" "KeepWorld" "KeepWorld")))
        (`BlackboardComponent.SetValueAsInt` _returnvalue "Hit?" (+ (`BlackboardComponent.GetValueAsInt` _returnvalue "Hit?") 1))
        (`BlackboardComponent.SetValueAsEnum` _returnvalue "AttackType" AttackType)
        (`BlackboardComponent.SetValueAsVector` _returnvalue "HitLocation" HitLocation)))))

(event `PlayHitMontage`
  (params (AttackType :type "/Game/ColdWinterWind/Blueprint/Enum/E_Attack Enum" :default "NewEnumerator0") (BTTask :type "BTTask_BlueprintBase Object Reference"))
  (bind _mesh (`self.Mesh`))
  (bind _mesh_2 (`self.Mesh`))
  (switch `/Game/ColdWinterWind/Blueprint/Enum/E_Attack` AttackType
    (:`NewEnumerator0`
      (`|PlayMontage` _mesh "/Game/ColdWinterWind/Animation/Montage/Enemy/Boss/HitMontage.HitMontage" 1.0 0.0 "Hit1"
        (:`OnCompleted`
          _)))
    (:`NewEnumerator1`
      (`|PlayMontage` _mesh "/Game/ColdWinterWind/Animation/Montage/Enemy/Boss/HitMontage.HitMontage" 1.0 0.0 "Hit2"
        (:`OnCompleted`
          _)))
    (:`NewEnumerator2`
      (`|PlayMontage` _mesh_2 "/Game/ColdWinterWind/Animation/Montage/Enemy/Boss/HitMontage.HitMontage" 1.0 0.0 "Hit3"
        (:`OnCompleted`
          _)))
    (:`NewEnumerator3`
      (`|PlayMontage` _mesh_2 "/Game/ColdWinterWind/Animation/Montage/Enemy/Boss/HitMontage.HitMontage" 1.0 0.0 "Hit4"
        (:`OnCompleted`
          _))))
  (`BlackboardComponent.SetValueAsInt` (`AIBlueprintHelperLibrary.GetBlackboard` null) "Hit?" -1)
  (`self.K2_DetachFromActor` "KeepWorld" "KeepWorld" "KeepWorld")
  (`BTTask_BlueprintBase.FinishExecute` BTTask false))

(event `PlayDeathMontage`
  (`|PlayMontage` (`self.Mesh`) "/Game/ColdWinterWind/Animation/Montage/Enemy/Boss/HitMontage.HitMontage" 1.0 0.0 "Death"))

(event `ReleaseMagic`
  (params (MagicType :type "/Game/ColdWinterWind/Blueprint/Enum/Skill/E_MagicType Enum" :default "NewEnumerator0"))
  (bind (_returnvalue_x _returnvalue_y _returnvalue_z) (`KismetMathLibrary.BreakVector` (`self.K2_GetActorLocation`)))
  (bind (_returnvalue_x_2 _returnvalue_y_2 _returnvalue_z_2) (`KismetMathLibrary.BreakVector` (`self.K2_GetActorLocation`)))
  (bind (_returnvalue_x_3 _returnvalue_y_3 _returnvalue_z_3) (`KismetMathLibrary.BreakVector` (`self.K2_GetActorLocation` (`GameplayStatics.GetPlayerCharacter` 0))))
  (bind (_returnvalue_x_4 _returnvalue_y_4 _returnvalue_z_4) (`KismetMathLibrary.BreakVector` (`self.K2_GetActorLocation` (`GameplayStatics.GetPlayerCharacter` 0))))
  (bind (_returnvalue_x_5 _returnvalue_y_5 _returnvalue_z_5) (`KismetMathLibrary.BreakVector` (`self.K2_GetActorLocation` (`GameplayStatics.GetPlayerCharacter` 0))))
  (switch `/Game/ColdWinterWind/Blueprint/Enum/Skill/E_MagicType` MagicType
    (:`NewEnumerator0`
      (`|SpawnActorFromClass` "/Game/ColdWinterWind/Blueprint/EnemyClass/BaseEnemyCharacter/BaseBossClass/Boss1/BP_Wind.BP_Wind_C" (`KismetMathLibrary.MakeTransform` (`KismetMathLibrary.MakeVector` _returnvalue_x_2 _returnvalue_y_2 (- _returnvalue_z_2 140.0))) "AlwaysSpawn" "OverrideRootScale" null null))
    (:`NewEnumerator1`
      (`|SpawnActorFromClass` "/Game/ColdWinterWind/Blueprint/EnemyClass/BaseEnemyCharacter/BaseBossClass/Boss1/BP_FireCircle.BP_FireCircle_C" (`KismetMathLibrary.MakeTransform` (`KismetMathLibrary.MakeVector` _returnvalue_x _returnvalue_y (- _returnvalue_z 140.0))) "AlwaysSpawn" "OverrideRootScale" null null))
    (:`NewEnumerator2`
      (`|SpawnActorFromClass` "/Game/ColdWinterWind/Blueprint/EnemyClass/BaseEnemyCharacter/BaseBossClass/Boss1/BP_lightning.BP_Lightning_C" (`KismetMathLibrary.MakeTransform` (`KismetMathLibrary.MakeVector` _returnvalue_x_4 _returnvalue_y_4 (- _returnvalue_z_4 82.0))) "Undefined" "OverrideRootScale" null null)
      (`KismetSystemLibrary.Delay` 0.5)
      (`|SpawnActorFromClass` "/Game/ColdWinterWind/Blueprint/EnemyClass/BaseEnemyCharacter/BaseBossClass/Boss1/BP_lightning.BP_Lightning_C" (`KismetMathLibrary.MakeTransform` (`KismetMathLibrary.MakeVector` _returnvalue_x_5 _returnvalue_y_5 (- _returnvalue_z_5 82.0))) "Undefined" "OverrideRootScale" null null)
      (`KismetSystemLibrary.Delay` 0.5)
      (`|SpawnActorFromClass` "/Game/ColdWinterWind/Blueprint/EnemyClass/BaseEnemyCharacter/BaseBossClass/Boss1/BP_lightning.BP_Lightning_C" (`KismetMathLibrary.MakeTransform` (`KismetMathLibrary.MakeVector` _returnvalue_x_3 _returnvalue_y_3 (- _returnvalue_z_3 82.0))) "Undefined" "OverrideRootScale" null null))))

(fn `GetBehaviorStatus`
  (params (BTTTask :type "/Game/ColdWinterWind/Blueprint/EnemyClass/BaseEnemyBehaviorTree/Boss1/BTT_BehaviorStatus Object Reference") (Player :type "/Game/ColdWinterWind/Blueprint/PlayerClass/Character/BP_BasicCharacter Object Reference"))
  (locals (RandomRange :type "Float (double-precision)" :default 10.0) (MontageAttack :type "Array of Name") (MontageMove :type "Array of Name"))
  (if (and (>= (`KismetMathLibrary.RandomIntegerInRange` 0 (`KismetMathLibrary.FTrunc` (+ (* (- 1.0 (/ (`self.HP`) (`self.MaxHP`))) (`local.RandomRange`)) 9.0))) 5) (not (`/Game/ColdWinterWind/Blueprint/PlayerClass/Character/BP_BasicCharacter.IsFall?` Player)))
    (`/Game/ColdWinterWind/Blueprint/EnemyClass/BaseEnemyBehaviorTree/Boss1/BTT_BehaviorStatus.Finished` BTTTask (`|GetArrayItem` (`self.MontageArray`)) (`|GetArrayItem` (`local.MontageAttack`) (`KismetMathLibrary.RandomIntegerInRange` 0 4)))
    (else
      (`/Game/ColdWinterWind/Blueprint/EnemyClass/BaseEnemyBehaviorTree/Boss1/BTT_BehaviorStatus.Finished` BTTTask (`|GetArrayItem` (`self.MontageArray`) 1) (`|GetArrayItem` (`local.MontageMove`) (`KismetMathLibrary.RandomIntegerInRange` 0 2))))))

(fn `UserConstructionScript`
  (`parent.UserConstructionScript`))