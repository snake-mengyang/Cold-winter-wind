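; BP_FireCircle is a timed area attack, filed under Boss1, that detonates once where it is placed.
; Five seconds after BeginPlay, it runs a stationary multi-sphere trace on the Visibility channel around itself.
; Each hit that casts to BP_BasicCharacter receives an AttackMessage with fixed damage, but the first failed cast stops the handling.
; It then spawns a double-scale shield-slam AOE emitter at its particle component and destroys itself.
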(event `self.ReceiveBeginPlay`
  (bind _returnvalue (`self.K2_GetActorLocation`))
  (bind (_returnvalue_location _returnvalue_rotation _returnvalue_scale) (`KismetMathLibrary.BreakTransform` (`SceneComponent.K2_GetComponentToWorld` (`self.ParticleSystem`))))
  (`KismetSystemLibrary.Delay` 5.0)
  (bind _outhits (`KismetSystemLibrary.SphereTraceMulti` _returnvalue _returnvalue 1200.0 "TraceTypeQuery1" true))
  (for _array_element _outhits
    (bind _asbp_basic_character (cast `/Game/ColdWinterWind/Blueprint/PlayerClass/Character/BP_BasicCharacter` (`.HitActor` (`GameplayStatics.BreakHitResult` _array_element))))
    (message `/Game/ColdWinterWind/Blueprint/Interface/BPI_AttackState.Attack` _asbp_basic_character "NewEnumerator3" -40.0 (`self.K2_GetActorLocation`) null false (0.0 0.0 0.0)))
  (`GameplayStatics.SpawnEmitterAtLocation` "/Game/InfinityBladeEffects/Effects/FX_Monsters/FX_Monster_Ausar/P_AU_ShieldSlam_AOE.P_AU_ShieldSlam_AOE" _returnvalue_location _returnvalue_rotation (* _returnvalue_scale 2))
  (`self.K2_DestroyActor`))

(fn `UserConstructionScript`)