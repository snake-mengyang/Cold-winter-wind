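; BP_Boss1AIController is the AI controller for the Boss1 enemy.
; On BeginPlay it casts its pawn to BP_Boss1Character, runs the Boss1 behavior tree, and seeds the blackboard with the spawn location as origin and a fixed radius.
; Its FindPlayer event flags that an enemy is found and stores the player reference on the blackboard.
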(event `self.ReceiveBeginPlay`
  (bind _returnvalue (`AIBlueprintHelperLibrary.GetBlackboard` null))
  (`parent.ReceiveBeginPlay`)
  (bind _asbp_boss_1character (cast `/Game/ColdWinterWind/Blueprint/EnemyClass/BaseEnemyCharacter/BaseBossClass/Boss1/BP_Boss1Character` (`self.K2_GetPawn`)))
  (set `self.CharacterRef` _asbp_boss_1character)
  (`self.RunBehaviorTree` "/Game/ColdWinterWind/Blueprint/EnemyClass/BaseEnemyBehaviorTree/Boss1/Boss1BehaviorTree.Boss1BehaviorTree")
  (`BlackboardComponent.SetValueAsVector` _returnvalue "OriginLocation" (`self.K2_GetActorLocation` (`self.CharacterRef`)))
  (`BlackboardComponent.SetValueAsFloat` _returnvalue "Radius" 2000.0))

(event `FindPlayer`
  (params (PlayerRef :type "/Game/ColdWinterWind/Blueprint/PlayerClass/Character/BP_BasicCharacter Object Reference"))
  (bind _returnvalue (`AIBlueprintHelperLibrary.GetBlackboard` null))
  (`BlackboardComponent.SetValueAsBool` _returnvalue "IsFindEnemy?" true)
  (`BlackboardComponent.SetValueAsObject` _returnvalue "PlayerRef" PlayerRef))

(fn `UserConstructionScript`
  (`parent.UserConstructionScript`))